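; Door Blueprint that swings its Door mesh open or closed through the OpenDoor event.
; OpenDoor plays or reverses DoorTimeline depending on IsDoorOpen, scaling the timeline track by OpenAngle to set relative yaw, and flips the flag on finish.
; BeginPlay sets the timeline time through SetTimeOfDoor and has the MaterialChanger apply the starting material to the mesh.
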(event `self.ReceiveBeginPlay`
  (`self.SetTimeOfDoor` (`self.IsDoorOpen`))
  (`/Game/MyAssets/Components/MaterialChanger.Change Material` (`self.MaterialChanger`) (`self.Door`) (`self.StartMaterialInt`)))

(event `OpenDoor`
  (bind _isdooropen (`self.IsDoorOpen`))
  (if (not (`self.IsDoorOpen`))
    (if (not _isdooropen)
      (bind (_direction _doorrotator) (`Timeline|DoorTimeline` :`NewTime` (`KismetMathLibrary.SelectFloat` (`TimelineComponent.GetTimelineLength` (`self.DoorTimeline`)) 0.0 (stale `SetTimeOfDoor` IsDoorOpen)) :!label _label)
        (:`Update`
          (`SceneComponent.K2_SetRelativeRotation` (`self.Door`) (`KismetMathLibrary.MakeRotator` 0.0 0.0 (* _doorrotator (`self.OpenAngle`))) false false))
        (:`Finished`
          (set `self.IsDoorOpen` (not (`self.IsDoorOpen`))))))
    (elif _isdooropen
      (goto _label :!via `Reverse`))))

(event `SetTimeOfDoor`
  (params (IsDoorOpen :type Boolean))
  (goto _label :!via `SetNewTime`))

(fn `UserConstructionScript`)