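; zMoveLong_BP is a level component actor that moves along a timeline-driven offset from its starting position, apparently on the Z axis.
; On BeginPlay it stores its location and plays the Movement_Positive_Negative timeline, whose ZMovement track scales ResultMaxDistance into that offset.
; Each update sets the location directly, without sweeping.
; A separate SetMoveSpeed event applies PlayRateMod as the timeline's play rate.
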(event `self.ReceiveBeginPlay`
  (set `self.StartPosition` (`self.K2_GetActorLocation`))
  (bind (_direction _zmovement) (`Timeline|Movement_Positive_Negative`)
    (:`Update`
      (`self.K2_SetActorLocation` (+ (`self.StartPosition`) (* (`self.ResultMaxDistance`) _zmovement))))))

(event `SetMoveSpeed`
  (`TimelineComponent.SetPlayRate` (`self.Movement_Positive_Negative`) (`self.PlayRateMod`)))

(fn `UserConstructionScript`)