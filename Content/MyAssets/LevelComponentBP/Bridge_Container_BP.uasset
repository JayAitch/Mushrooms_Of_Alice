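; Bridge container Blueprint that configures its attached zMoveLong_BP moving pieces as a group at BeginPlay.
; It loops over attached actors, casts each to zMoveLong_BP and multiplies its play rate modifier by the container's TargetPlayRate.
; Each piece gets the container's MaxDistance with a sign alternating by array index, so consecutive pieces receive opposite travel distances, then its move speed is set.
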(event `self.ReceiveBeginPlay`
  (for (_array_element _array_index) (`self.GetAttachedActors`)
    (bind _asz_move_long_bp (cast `/Game/MyAssets/LevelComponentBP/zMoveLong_BP` _array_element))
    (set `self.MovingComponent` _asz_move_long_bp)
    (set `/Game/MyAssets/LevelComponentBP/zMoveLong_BP.PlayRateMod` (* (`self.TargetPlayRate`) (`/Game/MyAssets/LevelComponentBP/zMoveLong_BP.PlayRateMod` _asz_move_long_bp)) _asz_move_long_bp)
    (set `/Game/MyAssets/LevelComponentBP/zMoveLong_BP.ResultMaxDistance` (* (`self.MaxDistance`) (* (`KismetMathLibrary.MultiplyMultiply_FloatFloat` -1.0 (`KismetMathLibrary.Conv_IntToDouble` _array_index)) 1.0)) (`self.MovingComponent`))
    (`/Game/MyAssets/LevelComponentBP/zMoveLong_BP.SetMoveSpeed` (`self.MovingComponent`))))

(fn `UserConstructionScript`)