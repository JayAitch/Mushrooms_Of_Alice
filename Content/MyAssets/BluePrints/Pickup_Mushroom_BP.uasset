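; Mushroom pickup actor that changes the player character's size on overlap.
; On BeginPlay, MaterialChanger sets the mushroom mesh's material from PickUpType.
; When an overlapping actor's class is exactly ThirdPersonCharacter, it passes PickUpType and that character to the CustomGI game instance's ChangeCharacterSize.
; The actor does not destroy or hide itself in this graph.
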(event `self.ReceiveBeginPlay`
  (`/Game/MyAssets/Components/MaterialChanger.Change Material` (`self.MaterialChanger`) (`self.MushroomStaticMesh`) (`self.PickUpType`)))

(event `self.ReceiveActorBeginOverlap`
  (params (OtherActor :type "Actor Object Reference"))
  (bind _output_get (set `self.CollidingActor` OtherActor))
  (if (== "/Game/ThirdPersonBP/Blueprints/ThirdPersonCharacter.ThirdPersonCharacter_C" (`GameplayStatics.GetObjectClass` _output_get))
    (bind _ascustom_gi (cast `/Game/Levels/CustomGI` (`GameplayStatics.GetGameInstance`)))
    (`/Game/Levels/CustomGI.ChangeCharacterSize` _ascustom_gi (`self.PickUpType`) (`self.CollidingActor`))))

(fn `UserConstructionScript`)